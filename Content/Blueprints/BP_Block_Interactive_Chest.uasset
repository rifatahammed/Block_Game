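; Interactive chest block Blueprint that opens and closes when its Interact event fires.
; A FlipFlop alternates between playing and reversing the OpenChest timeline on each interaction.
; The timeline's float track drives the relative pitch of PivotEmpty, swinging the chest around that pivot.
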(event EventBeginPlay
  (|CallParentFunction) ; This node is disabled and will not be called.\nDrag off pins to build functionality.
)

(event Collision|EventActorBeginOverlap
  (params (OtherActor :type Actor%20Object%20Reference))
  (|CallParentFunction OtherActor) ; This node is disabled and will not be called.\nDrag off pins to build functionality.
)

(event EventTick
  (params (DeltaSeconds :type Float%20%28single-precision%29))
  (|CallParentFunction DeltaSeconds) ; This node is disabled and will not be called.\nDrag off pins to build functionality.
)

(event EventInteract
  (Utilities|FlowControl|FlipFlop
    (:A
      (bind _newtrack_0 (Timeline|OpenChest Play)
        (:Update
          (Transformation|SetRelativeRotation (Variables|Default|GetPivotEmpty) (Math|Rotator|MakeRotator 0.0 _newtrack_0 0.0) false false))))
    (:B
      (Timeline|OpenChest Reverse))))

(fn ConstructionScript
  (|CallParentFunction))