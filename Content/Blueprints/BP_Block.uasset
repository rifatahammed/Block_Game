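; BP_Block is a destructible block actor that can be broken over time and removes itself when the breaking completes.
; On BeginPlay it creates a dynamic material instance from the block mesh's material.
; StartDestroy plays a timeline that drives the material's DestroyAmount parameter and destroys the actor when it finishes.
; StopDestroy stops the timeline and resets the parameter, so an interrupted break starts over from the beginning.
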(event Custom|StopDestroy
  (Rendering|Material|SetScalarParameterValue (Variables|Default|GetBlockMat) "DestroyAmount" 0.0 :!class /Script/Engine.MaterialInstanceDynamic)
  (bind _destroyamount (Timeline|DestroyTimeline Stop)
    (:Update
      (Rendering|Material|SetScalarParameterValue (Variables|Default|GetBlockMat) "DestroyAmount" _destroyamount :!class /Script/Engine.MaterialInstanceDynamic))
    (:Finished
      (Actor|DestroyActor))))

(event Custom|StartDestroy
  (bind _destroyamount (Timeline|DestroyTimeline PlayFromStart)
    (:Update
      (Rendering|Material|SetScalarParameterValue (Variables|Default|GetBlockMat) "DestroyAmount" _destroyamount :!class /Script/Engine.MaterialInstanceDynamic))
    (:Finished
      (Actor|DestroyActor))))

(event EventBeginPlay
  (bind _block (Variables|Default|GetBlock))
  (bind _returnvalue (Rendering|Material|CreateDynamicMaterialInstance _block 0 (Rendering|Material|GetMaterial _block 0) "None" :!class /Script/Engine.PrimitiveComponent))
  (Variables|Default|SetBlockMat _returnvalue))

(fn ConstructionScript)